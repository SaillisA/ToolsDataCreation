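; Base furniture actor (meuble) that the third-person character can target when inside its interaction area.
; The construction script configures it from a DataAsset: mesh, optional material override, interaction box transform and optional mesh transform.
; AppliquerDataAsset repeats that same setup as a callable function.
; Overlapping InteractibleArea sets the character's ObjetZone to this actor, and leaving clears it, both only while the character's MainLibre flag is true.
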(event OnComponentBeginOverlap(InteractibleArea)
  (params (OverlappedComponent :type Primitive%20Component%20Object%20Reference) (OtherActor :type Actor%20Object%20Reference) (OtherComp :type Primitive%20Component%20Object%20Reference) (OtherBodyIndex :type Integer) (bFromSweep :type Boolean) (SweepResult :type Hit%20Result%20Structure%20%28by%20ref%29))
  (bind _asbp_third_person_character (Utilities|Casting|CastToBP_ThirdPersonCharacter OtherActor))
  (if (Variables|/Game/Infiltration/Blueprints/Player/BP_ThirdPersonCharacter.BP_ThirdPersonCharacter_C|GetMainLibre _asbp_third_person_character)
    (Variables|/Game/Infiltration/Blueprints/Player/BP_ThirdPersonCharacter.BP_ThirdPersonCharacter_C|SetObjetZone _asbp_third_person_character self)))

(event OnComponentEndOverlap(InteractibleArea)
  (params (OverlappedComponent :type Primitive%20Component%20Object%20Reference) (OtherActor :type Actor%20Object%20Reference) (OtherComp :type Primitive%20Component%20Object%20Reference) (OtherBodyIndex :type Integer))
  (bind _asbp_third_person_character (Utilities|Casting|CastToBP_ThirdPersonCharacter OtherActor))
  (if (Variables|/Game/Infiltration/Blueprints/Player/BP_ThirdPersonCharacter.BP_ThirdPersonCharacter_C|GetMainLibre _asbp_third_person_character)
    (Variables|/Game/Infiltration/Blueprints/Player/BP_ThirdPersonCharacter.BP_ThirdPersonCharacter_C|SetObjetZone _asbp_third_person_character 0)))

(event EventBeginPlay)

(event Collision|EventActorBeginOverlap
  (params (OtherActor :type Actor%20Object%20Reference)))

(event EventTick
  (params (DeltaSeconds :type Float%20%28single-precision%29)))

(fn ConstructionScript
  (Components|StaticMesh|SetStaticMesh (Variables|Default|GetMeshDefault) (Variables|/Game/Meubles/Data_Assets_Meubles/BP_PrimayDataAssetsMeubles.BP_PrimayDataAssetsMeubles_C|GetObjetMesh (Variables|Default|GetDataAsset)))
  (if (== (Variables|/Game/Meubles/Data_Assets_Meubles/BP_PrimayDataAssetsMeubles.BP_PrimayDataAssetsMeubles_C|GetMaterial (Variables|Default|GetDataAsset)) 0)
    _
    (else
      (Rendering|Material|SetMaterial (Variables|Default|GetMeshDefault) 0 (Variables|/Game/Meubles/Data_Assets_Meubles/BP_PrimayDataAssetsMeubles.BP_PrimayDataAssetsMeubles_C|GetMaterial (Variables|Default|GetDataAsset)))))
  (Transformation|SetRelativeTransform (Variables|Default|GetInteractibleArea) (Variables|/Game/Meubles/Data_Assets_Meubles/BP_PrimayDataAssetsMeubles.BP_PrimayDataAssetsMeubles_C|GetInteractableArea (Variables|Default|GetDataAsset)) false false)
  (if (not (== (Variables|/Game/Meubles/Data_Assets_Meubles/BP_PrimayDataAssetsMeubles.BP_PrimayDataAssetsMeubles_C|GetMeshTransform (Variables|Default|GetDataAsset)) (Variables|Default|GettransformBlank)))
    (Transformation|SetRelativeTransform (Variables|Default|GetMeshDefault) (Variables|/Game/Meubles/Data_Assets_Meubles/BP_PrimayDataAssetsMeubles.BP_PrimayDataAssetsMeubles_C|GetMeshTransform (Variables|Default|GetDataAsset)) false false)))

(fn AppliquerDataAsset
  (Components|StaticMesh|SetStaticMesh (Variables|Default|GetMeshDefault) (Variables|/Game/Meubles/Data_Assets_Meubles/BP_PrimayDataAssetsMeubles.BP_PrimayDataAssetsMeubles_C|GetObjetMesh (Variables|Default|GetDataAsset)))
  (if (== (Variables|/Game/Meubles/Data_Assets_Meubles/BP_PrimayDataAssetsMeubles.BP_PrimayDataAssetsMeubles_C|GetMaterial (Variables|Default|GetDataAsset)) 0)
    _
    (else
      (Rendering|Material|SetMaterial (Variables|Default|GetMeshDefault) 0 (Variables|/Game/Meubles/Data_Assets_Meubles/BP_PrimayDataAssetsMeubles.BP_PrimayDataAssetsMeubles_C|GetMaterial (Variables|Default|GetDataAsset)))))
  (Transformation|SetRelativeTransform (Variables|Default|GetInteractibleArea) (Variables|/Game/Meubles/Data_Assets_Meubles/BP_PrimayDataAssetsMeubles.BP_PrimayDataAssetsMeubles_C|GetInteractableArea (Variables|Default|GetDataAsset)) false false)
  (if (not (== (Variables|/Game/Meubles/Data_Assets_Meubles/BP_PrimayDataAssetsMeubles.BP_PrimayDataAssetsMeubles_C|GetMeshTransform (Variables|Default|GetDataAsset)) (Variables|Default|GettransformBlank)))
    (Transformation|SetRelativeTransform (Variables|Default|GetMeshDefault) (Variables|/Game/Meubles/Data_Assets_Meubles/BP_PrimayDataAssetsMeubles.BP_PrimayDataAssetsMeubles_C|GetMeshTransform (Variables|Default|GetDataAsset)) false false)))