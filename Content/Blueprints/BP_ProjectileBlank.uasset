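; BP_ProjectileBlank is a projectile actor configured from a chosen data asset, with no gameplay logic in its event graph.
; Its construction script sets the Cube component's mesh from DataAssetChoisis and copies name, heavy flag, color and projectile type into its own variables.
; The color is only stored in ColorMesh, as this graph does not apply it to a material.
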(event EventBeginPlay)

(event Collision|EventActorBeginOverlap
  (params (OtherActor :type Actor%20Object%20Reference)))

(event EventTick
  (params (DeltaSeconds :type Float%20%28single-precision%29)))

(fn ConstructionScript
  (bind _dataassetchoisis (Variables|Var|GetDataAssetChoisis))
  (Components|StaticMesh|SetStaticMesh (Variables|Default|GetCube) (Variables|/Game/Blueprints/BP_DataAssetPrimary_Test.BP_DataAssetPrimary_Test_C|GetMesh _dataassetchoisis))
  (Variables|Var|SetProjName (Variables|/Game/Blueprints/BP_DataAssetPrimary_Test.BP_DataAssetPrimary_Test_C|GetName _dataassetchoisis))
  (Variables|Var|SetHeavy (Variables|/Game/Blueprints/BP_DataAssetPrimary_Test.BP_DataAssetPrimary_Test_C|GetIsHeavy _dataassetchoisis))
  (Variables|Var|SetColorMesh (Variables|/Game/Blueprints/BP_DataAssetPrimary_Test.BP_DataAssetPrimary_Test_C|GetColor _dataassetchoisis))
  (Variables|Var|SetProjType (Variables|/Game/Blueprints/BP_DataAssetPrimary_Test.BP_DataAssetPrimary_Test_C|GetTypeProjectile _dataassetchoisis)))