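; AI controller for the weak guard in the infiltration game, running its behavior tree and seeding the blackboard with start position, rotation and alive state.
; Sight perception sets or clears the player as TargetActor and stores the last seen location when lost.
; Tick also writes the player's true location to the blackboard every frame.
; A knockout event marks the guard not alive and fakes the fall by rolling and lowering the pawn.
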(event OnTargetPerceptionUpdated(AIPerception)
  (params (Actor :type Actor%20Object%20Reference) (Stimulus :type AI%20Stimulus%20Structure))
  (CallFunction|VisionJoueur Actor Stimulus))

(event Custom|SeFaitAssomer
  (Development|PrintString "PAF")
  (CallFunction|EstAssommer))

(event EventBeginPlay
  (bind _self self)
  (AI|RunBehaviorTree "/Game/Infiltration/AI/AI_GuardFaible/BT_BehaviourTreeGuardFaible.BT_BehaviourTreeGuardFaible")
  (bind _blackboardcomponent (Class|AIController|UseBlackboard "/Game/Infiltration/AI/AI_GuardFaible/BB_BlackBoardAIGuardFaible.BB_BlackBoardAIGuardFaible"))
  (Variables|Default|SetBlackboard%20Component _blackboardcomponent)
  (AI|Components|Blackboard|SetValueasVector (Variables|Default|GetBlackboard%20Component) (Utilities|Name|MakeLiteralName "PositionInitial") (Transformation|GetActorLocation _self))
  (Class|BlackboardComponent|SetValueasRotator (Variables|Default|GetBlackboard%20Component) (Utilities|Name|MakeLiteralName "RotationInitial") (Transformation|GetActorRotation _self))
  (AI|Components|Blackboard|SetValueasBool (Variables|Default|GetBlackboard%20Component) (Utilities|Name|MakeLiteralName "EstVivant") true)
  (bind _asbp_aicharacter_guard_faible (Utilities|Casting|CastToBP_AICharacterGuardFaible (Pawn|GetControlledPawn)))
  (Variables|/Game/Infiltration/AI/AI_GuardFaible/BP_AICharacterGuardFaible.BP_AICharacterGuardFaible_C|SetAifeur _asbp_aicharacter_guard_faible self))

(event EventTick
  (params (DeltaSeconds :type Float%20%28single-precision%29))
  (AI|Components|Blackboard|SetValueasVector (Variables|Default|GetBlackboard%20Component) (Utilities|Name|MakeLiteralName "PlayerLocation") (Transformation|GetActorLocation (Game|GetPlayerCharacter 0))))

(fn ConstructionScript)

(fn EstAssommer
  (bind _returnvalue (Pawn|GetControlledPawn))
  (bind _returnvalue_2 (Transformation|GetActorRotation _returnvalue))
  (bind _returnvalue_3 (Transformation|GetActorLocation _returnvalue))
  (Development|PrintString "Im dead")
  (AI|Components|Blackboard|SetValueasBool (Variables|Default|GetBlackboard%20Component) (Utilities|Name|MakeLiteralName "EstVivant") false)
  (Transformation|SetActorRotation _returnvalue (Math|Rotator|MakeRotator -9e+01 (.pitch _returnvalue_2) (.yaw _returnvalue_2)))
  (Transformation|SetActorLocation _returnvalue (Math|Vector|MakeVector (.x _returnvalue_3) (.y _returnvalue_3) -18.0) false false))

(fn VisionJoueur
  (params (Joueur :type Actor%20Object%20Reference) (Sens :type AI%20Stimulus%20Structure))
  (bind _returnvalue (Class|AIPerceptionSystem|GetSenseClassforStimulus Sens))
  (if (== _returnvalue "/Script/AIModule.AISense_Sight")
    (if (== Joueur (Game|GetPlayerCharacter 0))
      (AI|Components|Blackboard|SetValueasObject (Variables|Default|GetBlackboard%20Component) (Utilities|Name|MakeLiteralName "TargetActor") (Utilities|SelectObject (Game|GetPlayerCharacter 0) 0 (.bsuccessfullysensed Sens)))
      (if (not (.bsuccessfullysensed Sens))
        (AI|Components|Blackboard|SetValueasVector (Variables|Default|GetBlackboard%20Component) (Utilities|Name|MakeLiteralName "DernierePositionJoueur") (.stimuluslocation Sens)))
      (else
        (return)))
    (else
      (return))))