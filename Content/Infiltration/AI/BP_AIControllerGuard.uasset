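; AI controller for guards in the Infiltration game, running the guard behavior tree and feeding its blackboard.
; Tick writes the player's actual location to PlayerLocation every frame, regardless of perception.
; AI Perception updates pass to VisionJoueur, which handles only sight of the player character.
; It sets TargetActor while the player is seen, and on sight loss clears it and stores the stimulus location as DernierePositionJoueur.
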(event OnTargetPerceptionUpdated(AIPerception)
  (params (Actor :type Actor%20Object%20Reference) (Stimulus :type AI%20Stimulus%20Structure))
  (CallFunction|VisionJoueur Actor Stimulus))

(event EventBeginPlay
  (AI|RunBehaviorTree "/Game/Infiltration/AI/BT_BehaviourTreeGuard.BT_BehaviourTreeGuard")
  (bind _blackboardcomponent (Class|AIController|UseBlackboard "/Game/Infiltration/AI/BB_BlackBoardIAGuard.BB_BlackBoardIAGuard"))
  (Variables|Default|SetBlackBoardVar _blackboardcomponent))

(event EventTick
  (params (DeltaSeconds :type Float%20%28single-precision%29))
  (AI|Components|Blackboard|SetValueasVector (Variables|Default|GetBlackBoardVar) (Utilities|Name|MakeLiteralName "PlayerLocation") (Transformation|GetActorLocation (Game|GetPlayerCharacter 0))))

(fn ConstructionScript)

(fn VisionJoueur
  (params (Joueur :type Actor%20Object%20Reference) (Sens :type AI%20Stimulus%20Structure))
  (bind _returnvalue (Class|AIPerceptionSystem|GetSenseClassforStimulus Sens))
  (if (== _returnvalue "/Script/AIModule.AISense_Sight")
    (if (== Joueur (Game|GetPlayerCharacter 0))
      (AI|Components|Blackboard|SetValueasObject (Variables|Default|GetBlackboard) (Utilities|Name|MakeLiteralName "TargetActor") (Utilities|SelectObject (Game|GetPlayerCharacter 0) 0 (.bsuccessfullysensed Sens)))
      (if (not (.bsuccessfullysensed Sens))
        (AI|Components|Blackboard|SetValueasVector (Variables|Default|GetBlackboard) (Utilities|Name|MakeLiteralName "DernierePositionJoueur") (.stimuluslocation Sens)))
      (else
        (return)))
    (else
      (return))))