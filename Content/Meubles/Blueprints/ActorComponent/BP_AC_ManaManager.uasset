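; Actor component that tracks mana for the BP_ThirdPersonCharacter that owns it.
; On BeginPlay it reads the owner's player level, prints it, adds ten times that level to ManaMax and fills ManaActuel to that maximum.
; GagnePerdMana adds a signed value to current mana without clamping, and GetMana returns the current amount.
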(event EventBeginPlay
  (bind _asbp_third_person_character (Utilities|Casting|CastToBP_ThirdPersonCharacter (Components|GetOwner)))
  (bind _level (Default|GetPlayerLevel _asbp_third_person_character))
  (Development|PrintString (Utilities|String|ToString(Integer) _level))
  (bind _output_get (Variables|Default|SetNiveauMana _level))
  (bind _output_get_2 (Variables|Default|SetManaMax (+ (* _output_get 10) (Variables|Default|GetManaMax))))
  (Variables|Default|SetManaActuel _output_get_2))

(event EventTick
  (params (DeltaSeconds :type Float%20%28single-precision%29)))

(fn GagnePerdMana
  (params (Valeur :type Integer))
  (Variables|Default|SetManaActuel (+ Valeur (Variables|Default|GetManaActuel)))
  (if true
    (return)))

(fn GetMana
  (return (Variables|Default|GetManaActuel)))